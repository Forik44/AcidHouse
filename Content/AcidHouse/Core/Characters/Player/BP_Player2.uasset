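; BP_Player2 is a player character Blueprint that extends its parent's sprint start and end events.
; It plays SpringArmSprintTimeline forward on sprint start and reverses it on sprint end, after calling the parent.
; A Lerp meant to set the spring arm's TargetArmLength from the timeline is disconnected and has zeroed endpoints, so this graph never changes the camera distance.
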(event EventOnSprintStart
  (|CallParentFunction)
  (bind _value (Timeline|Spring%20arm%20sprint%20timeline Play)))

(event EventBeginPlay
  (|CallParentFunction))

(event EventOnSprintEnd
  (|CallParentFunction)
  (bind _value (Timeline|Spring%20arm%20sprint%20timeline Reverse)))

(fn ConstructionScript)