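; Knife weapon Blueprint that shows its static mesh only while equipped, hiding it on BeginPlay.
; An equipment state change event sets the mesh visibility and Visability locally, and an autonomous proxy owner also forwards the state through a server event.
; The server event applies the same state, and the OnRep for Visability updates the mesh when the replicated value arrives.
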(event Custom|OnEquipmentStateChangedEvent
  (params (bIsEquipped :type Boolean))
  (bind _returnvalue (Components|GetOwner))
  (Utilities|IsValid _returnvalue
    (:Is%20Valid
      (if (Utilities|Enum|Equal(Enum) (Networking|GetLocalRole _returnvalue) "ROLE_AutonomousProxy")
        (CallFunction|ServerEquipmentStateChanged bIsEquipped))
      (Rendering|SetVisibility (Variables|Default|GetStaticMesh) bIsEquipped false)
      (Variables|Default|SetVisability bIsEquipped))))

(event Custom|Server_EquipmentStateChanged
  (params (Visability :type Boolean))
  (Rendering|SetVisibility (Variables|Default|GetStaticMesh) Visability false)
  (Variables|Default|SetVisability Visability))

(event EventBeginPlay
  (EventDispatchers|BindEventtoOnEquipmentStateChanged (delegate Custom|OnEquipmentStateChangedEvent))
  (Rendering|SetVisibility (Variables|Default|GetStaticMesh) false false))

(fn ConstructionScript)

(fn OnRepVisability
  (Rendering|SetVisibility (Variables|Default|GetStaticMesh) (Variables|Default|GetVisability) false))